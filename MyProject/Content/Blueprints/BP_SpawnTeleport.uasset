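; BP_SpawnTeleport is a checkpoint actor that moves the player's respawn point to its own location.
; On BeginPlay it caches the third-person player character and writes its own transform to NewRespawnTrans in the BP_StoreVariables game instance.
; When that character overlaps its Box, it replaces the first PlayerStart found with one spawned at its transform.
; It then saves that transform to the game instance again.
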(event OnComponentBeginOverlap(Box)
  (params (OverlappedComponent :type Primitive%20Component%20Object%20Reference) (OtherActor :type Actor%20Object%20Reference) (OtherComp :type Primitive%20Component%20Object%20Reference) (OtherBodyIndex :type Integer) (bFromSweep :type Boolean) (SweepResult :type Hit%20Result%20Structure%20%28by%20ref%29))
  (bind _returnvalue (Transformation|GetActorTransform))
  (if (== OtherActor (Variables|Default|GetAs%20BP%20Third%20Person%20Character))
    (bind _returnvalue_2 (Actor|GetActorOfClass "/Script/Engine.PlayerStart"))
    (Actor|DestroyActor _returnvalue_2)
    (Game|SpawnActorfromClass "/Script/Engine.PlayerStart" _returnvalue "Undefined" 0 0)
    (bind _asbp_store_variables (Utilities|Casting|CastToBP_StoreVariables (Game|GetGameInstance)))
    (Variables|/Game/Blueprints/BP_StoreVariables.BP_StoreVariables_C|SetNewRespawnTrans _asbp_store_variables _returnvalue)))

(event EventBeginPlay
  (bind _asbp_third_person_character (Utilities|Casting|CastToBP_ThirdPersonCharacter (Game|GetPlayerCharacter 0)))
  (Variables|Default|SetAs%20BP%20Third%20Person%20Character _asbp_third_person_character)
  (bind _output_get (Variables|Default|SetRespawnTrans (Transformation|GetActorTransform)))
  (bind _asbp_store_variables (Utilities|Casting|CastToBP_StoreVariables (Game|GetGameInstance)))
  (Variables|/Game/Blueprints/BP_StoreVariables.BP_StoreVariables_C|SetNewRespawnTrans _asbp_store_variables _output_get))

(fn ConstructionScript)